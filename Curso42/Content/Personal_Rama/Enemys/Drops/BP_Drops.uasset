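; Currency pickup for enemy drops that represents one of four types (Dark Shards, Radiant Token, Burnt Crystal, Frost Crystal) through its Coins gameplay tags.
; The construction script applies a matching outline overlay material, while BeginPlay sets the gem mesh, material and light color.
; On overlap with any actor, without checking which, it destroys itself and increments the matching counter on the player's BP_TRON.
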(event `self.ReceiveBeginPlay`
  (`|ExecutionSequence`
    (:`then_0`
      (if (`BlueprintGameplayTagLibrary.HasTag` (`self.Coins`) (struct :`TagName` "Coins.DarkShards") true)
        (`PrimitiveComponent.SetMaterial` (`self.StaticMeshComponent`) 0 "/Game/Personal_Rama/Enemys/Drops/Materials/M_DarkShard.M_DarkShard")
        (`LightComponent.SetLightColor` (`self.Light`) (struct :`R` 0.050803 :`B` 0.15625 :`A` 1.0) true)
        (`StaticMeshComponent.SetStaticMesh` (`self.StaticMeshComponent`) "/Game/Personal_Rama/Enemys/Drops/CrystalsFBX/source/Gema1.Gema1")
        (set `self.Outline` "/Game/Personal_Rama/Enemys/Drops/Materials/M_Outline_Dark.M_Outline_Dark")))
    (:`then_1`
      (if (`BlueprintGameplayTagLibrary.HasTag` (`self.Coins`) (struct :`TagName` "Coins.RadiantToken") true)
        (`PrimitiveComponent.SetMaterial` (`self.StaticMeshComponent`) 0 "/Game/Personal_Rama/Enemys/Drops/Materials/M_RadiantToken.M_RadiantToken")
        (`LightComponent.SetLightColor` (`self.Light`) (struct :`R` 0.698907 :`G` 1.0 :`B` 0.479167 :`A` 1.0) true)
        (`StaticMeshComponent.SetStaticMesh` (`self.StaticMeshComponent`) "/Game/Personal_Rama/Enemys/Drops/CrystalsFBX/source/Gema2.Gema2")
        (set `self.Outline` "/Game/Personal_Rama/Enemys/Drops/Materials/M_Outline_Radiant.M_Outline_Radiant")))
    (:`then_2`
      (if (`BlueprintGameplayTagLibrary.HasTag` (`self.Coins`) (struct :`TagName` "Coins.BurntCrystal") true)
        (`PrimitiveComponent.SetMaterial` (`self.StaticMeshComponent`) 0 "/Game/Personal_Rama/Enemys/Drops/Materials/M_BurntCrystal.M_BurntCrystal")
        (`LightComponent.SetLightColor` (`self.Light`) (struct :`R` 1.0 :`G` 0.070808 :`A` 1.0) true)
        (`StaticMeshComponent.SetStaticMesh` (`self.StaticMeshComponent`) "/Game/Personal_Rama/Enemys/Drops/CrystalsFBX/source/Gema3.Gema3")
        (set `self.Outline` "/Game/Personal_Rama/Enemys/Drops/Materials/M_Outline_Burnt.M_Outline_Burnt")))
    (:`then_3`
      (if (`BlueprintGameplayTagLibrary.HasTag` (`self.Coins`) (struct :`TagName` "Coins.FrostCrystal") true)
        (`PrimitiveComponent.SetMaterial` (`self.StaticMeshComponent`) 0 "/Game/Personal_Rama/Enemys/Drops/Materials/M_FrostCrystal.M_FrostCrystal")
        (`LightComponent.SetLightColor` (`self.Light`) (struct :`G` 0.984722 :`B` 1.0 :`A` 1.0) true)
        (`StaticMeshComponent.SetStaticMesh` (`self.StaticMeshComponent`) "/Game/Personal_Rama/Enemys/Drops/CrystalsFBX/source/Gema3.Gema3")
        (set `self.Outline` "/Game/Personal_Rama/Enemys/Drops/Materials/M_Outline_Frost.M_Outline_Frost")))))

(event `self.ReceiveActorBeginOverlap`
  (params (OtherActor :type "Actor Object Reference"))
  (`|ExecutionSequence`
    (:`then_0`
      (if (`BlueprintGameplayTagLibrary.HasTag` (`self.Coins`) (struct :`TagName` "Coins.DarkShards") true)
        (`self.K2_DestroyActor`)
        (bind _asbp_tron (cast `/Game/carpeta_thiago/tron/BP_TRON` (`GameplayStatics.GetPlayerCharacter` 0)))
        (set `/Game/carpeta_thiago/tron/BP_TRON.DarkShards` (+ (`/Game/carpeta_thiago/tron/BP_TRON.DarkShards` _asbp_tron) 1) _asbp_tron)))
    (:`then_1`
      (if (`BlueprintGameplayTagLibrary.HasTag` (`self.Coins`) (struct :`TagName` "Coins.RadiantToken") true)
        (`self.K2_DestroyActor`)
        (bind _asbp_tron_2 (cast `/Game/carpeta_thiago/tron/BP_TRON` (`GameplayStatics.GetPlayerCharacter` 0)))
        (set `/Game/carpeta_thiago/tron/BP_TRON.RadiantToken` (+ (`/Game/carpeta_thiago/tron/BP_TRON.RadiantToken` _asbp_tron_2) 1) _asbp_tron_2)))
    (:`then_2`
      (if (`BlueprintGameplayTagLibrary.HasTag` (`self.Coins`) (struct :`TagName` "Coins.BurntCrystal") true)
        (`self.K2_DestroyActor`)
        (bind _asbp_tron_3 (cast `/Game/carpeta_thiago/tron/BP_TRON` (`GameplayStatics.GetPlayerCharacter` 0)))
        (set `/Game/carpeta_thiago/tron/BP_TRON.BurntCrystal` (+ (`/Game/carpeta_thiago/tron/BP_TRON.BurntCrystal` _asbp_tron_3) 1) _asbp_tron_3)))
    (:`then_3`
      (if (`BlueprintGameplayTagLibrary.HasTag` (`self.Coins`) (struct :`TagName` "Coins.FrostCrystal") true)
        (`self.K2_DestroyActor`)
        (bind _asbp_tron_4 (cast `/Game/carpeta_thiago/tron/BP_TRON` (`GameplayStatics.GetPlayerCharacter` 0)))
        (set `/Game/carpeta_thiago/tron/BP_TRON.FrostCrystal` (+ (`/Game/carpeta_thiago/tron/BP_TRON.FrostCrystal` _asbp_tron_4) 1) _asbp_tron_4)))))

(fn `UserConstructionScript`
  (`|ExecutionSequence`
    (:`then_0`
      (if (`BlueprintGameplayTagLibrary.HasTag` (`self.Coins`) (struct :`TagName` "Coins.DarkShards") true)
        (set `self.Outline` "/Game/Personal_Rama/Enemys/Drops/Materials/M_Outline_Dark.M_Outline_Dark")
        (`MeshComponent.SetOverlayMaterial` (`self.StaticMeshComponent`) (`self.Outline`) :!label _label)))
    (:`then_1`
      (if (`BlueprintGameplayTagLibrary.HasTag` (`self.Coins`) (struct :`TagName` "Coins.RadiantToken") true)
        (set `self.Outline` "/Game/Personal_Rama/Enemys/Drops/Materials/M_Outline_Radiant.M_Outline_Radiant")
        (goto _label)))
    (:`then_2`
      (if (`BlueprintGameplayTagLibrary.HasTag` (`self.Coins`) (struct :`TagName` "Coins.BurntCrystal") true)
        (set `self.Outline` "/Game/Personal_Rama/Enemys/Drops/Materials/M_Outline_Burnt.M_Outline_Burnt")
        (goto _label)))
    (:`then_3`
      (if (`BlueprintGameplayTagLibrary.HasTag` (`self.Coins`) (struct :`TagName` "Coins.FrostCrystal") true)
        (set `self.Outline` "/Game/Personal_Rama/Enemys/Drops/Materials/M_Outline_Frost.M_Outline_Frost")
        (goto _label)))))
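; Frost crystal drop pickup that adds one to the player character's DarkShards count when collected.
; A spawn cooldown set on BeginPlay counts down by a fixed step every Tick, so the delay depends on frame rate.
; Overlap by BP_ThirdPersonCharacter after the cooldown destroys the actor and credits player 0's character.
; The construction script applies a frost outline overlay material to the static mesh.
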(event `self.ReceiveBeginPlay`
  (set `self.SpawnCooldown` 5.0))

(event `self.ReceiveTick`
  (params (DeltaSeconds :type "Float (single-precision)"))
  (set `self.SpawnCooldown` (- (`self.SpawnCooldown`) 0.1)))

(event `self.ReceiveActorBeginOverlap`
  (params (OtherActor :type "Actor Object Reference"))
  (cast `/Game/ThirdPerson/Blueprints/BP_ThirdPersonCharacter` OtherActor)
  (if (<= (`self.SpawnCooldown`) 0.0)
    (`self.K2_DestroyActor`)
    (bind _asbp_third_person_character (cast `/Game/ThirdPerson/Blueprints/BP_ThirdPersonCharacter` (`GameplayStatics.GetPlayerCharacter` 0)))
    (set `/Game/ThirdPerson/Blueprints/BP_ThirdPersonCharacter.DarkShards` (+ (`/Game/ThirdPerson/Blueprints/BP_ThirdPersonCharacter.DarkShards` _asbp_third_person_character) 1) _asbp_third_person_character)))

(fn `UserConstructionScript`
  (set `self.Outline` "/Game/Personal_Rama/Enemys/Drops/Materials/M_Outline_Frost.M_Outline_Frost")
  (`MeshComponent.SetOverlayMaterial` (`self.StaticMeshComponent`) (`self.Outline`)))
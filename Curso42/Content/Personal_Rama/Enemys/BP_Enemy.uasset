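; Enemy Blueprint that sets its life and damage by level and takes damage from the player's hit checks.
; On BeginPlay, gameplay tags in LvlTags select one of six stat tiers across E_I and E_R groups.
; Overlapping a BP_HitCheck actor applies the player character's PlayerDamage to itself.
; AnyDamage subtracts that from EnemyLife and prints the result, with no death handling.
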(event `self.ReceiveActorBeginOverlap`
  (params (OtherActor :type "Actor Object Reference"))
  (bind _asbp_third_person_character (cast `/Game/ThirdPerson/Blueprints/BP_ThirdPersonCharacter` (`GameplayStatics.GetPlayerCharacter` 0)))
  (cast `/Game/Personal_Rama/Archives/BP_HitCheck` OtherActor)
  (`GameplayStatics.ApplyDamage` self (`KismetMathLibrary.Conv_IntToDouble` (`/Game/ThirdPerson/Blueprints/BP_ThirdPersonCharacter.PlayerDamage` _asbp_third_person_character))))

(event `self.ReceiveAnyDamage`
  (params (Damage :type "Float (single-precision)") (DamageType :type "DamageType Object Reference") (InstigatedBy :type "Controller Object Reference") (DamageCauser :type "Actor Object Reference"))
  (set `self.EnemyLife` (- (`self.EnemyLife`) Damage))
  (`KismetSystemLibrary.PrintString` (`KismetStringLibrary.Conv_IntToString` (`self.EnemyLife`))))

(event `self.ReceiveBeginPlay`
  ;[1 1 1 1 150] LVL
  (`|ExecutionSequence`
    (:`then_0`
      (if (`BlueprintGameplayTagLibrary.HasTag` (`self.LvlTags`) (struct :`TagName` "LVL_Enemy.E_I.LVL_1") true)
        (set `self.EnemyLife` 30)
        (set `self.EnemyDamage` 5)))
    (:`then_1`
      (if (`BlueprintGameplayTagLibrary.HasTag` (`self.LvlTags`) (struct :`TagName` "LVL_Enemy.E_I.LVL_2") true)
        (set `self.EnemyLife` 50)
        (set `self.EnemyDamage` 10)))
    (:`then_2`
      (if (`BlueprintGameplayTagLibrary.HasTag` (`self.LvlTags`) (struct :`TagName` "LVL_Enemy.E_I.LVL_3") true)
        (set `self.EnemyLife` 80)
        (set `self.EnemyDamage` 15)))
    (:`then_3`
      (if (`BlueprintGameplayTagLibrary.HasTag` (`self.LvlTags`) (struct :`TagName` "LVL_Enemy.E_R.LVL_4") true)
        (set `self.EnemyLife` 120)
        (set `self.EnemyDamage` 25)))
    (:`then_4`
      (if (`BlueprintGameplayTagLibrary.HasTag` (`self.LvlTags`) (struct :`TagName` "LVL_Enemy.E_R.LVL_5") true)
        (set `self.EnemyLife` 150)
        (set `self.EnemyDamage` 40)))
    (:`then_5`
      (if (`BlueprintGameplayTagLibrary.HasTag` (`self.LvlTags`) (struct :`TagName` "LVL_Enemy.E_R.LVL_6") true)
        (set `self.EnemyLife` 200)
        (set `self.EnemyDamage` 60)))))

(fn `UserConstructionScript`)
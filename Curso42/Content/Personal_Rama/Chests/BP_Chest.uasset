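; BP_Chest is a chest Blueprint that sets its loot tier from level gameplay tags.
; On BeginPlay, a Sequence checks the LvlTags container for exact matches of the five LVL_Chest level tags and writes the matching number into Loot.
; Each check runs independently, so the highest matching level wins; opening or spawning loot is not handled here.
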(event `self.ReceiveBeginPlay`
  (`|ExecutionSequence`
    (:`then_0`
      (if (`BlueprintGameplayTagLibrary.HasTag` (`self.LvlTags`) (struct :`TagName` "LVL_Chest.LVL_1") true)
        (set `self.Loot` 1)))
    (:`then_1`
      (if (`BlueprintGameplayTagLibrary.HasTag` (`self.LvlTags`) (struct :`TagName` "LVL_Chest.LVL_2") true)
        (set `self.Loot` 2)))
    (:`then_2`
      (if (`BlueprintGameplayTagLibrary.HasTag` (`self.LvlTags`) (struct :`TagName` "LVL_Chest.LVL_3") true)
        (set `self.Loot` 3)))
    (:`then_3`
      (if (`BlueprintGameplayTagLibrary.HasTag` (`self.LvlTags`) (struct :`TagName` "LVL_Chest.LVL_4") true)
        (set `self.Loot` 4)))
    (:`then_4`
      (if (`BlueprintGameplayTagLibrary.HasTag` (`self.LvlTags`) (struct :`TagName` "LVL_Chest.LVL_5") true)
        (set `self.Loot` 5)))))

(fn `UserConstructionScript`)